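; Enemy character that turns to face the player when pawn sensing spots them and fires at them.
; It spawns a BP_PlayerBullet, but hits come from two debug-drawn line traces: one finds a static-world aim point, the second checks what lies along that line.
; A player hit, after delays with sound and particles, destroys the bullet, applies damage, updates the HUD and triggers death at zero health.
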(event OnSeePawn(PawnSensing)
  (params (Pawn :type Pawn%20Object%20Reference))
  (bind _projectilespawnlocation (Variables|Default|GetProjectileSpawnLocation))
  (bind _projectilespawnlocation_2 (Variables|Default|GetProjectileSpawnLocation))
  (bind _returnvalue (Transformation|GetWorldLocation _projectilespawnlocation))
  ;[1 1 1] On Pawn Sence start firing and dealing damage
  (bind _asbp_my_player (Utilities|Casting|CastToBP_MyPlayer Pawn))
  (Variables|Default|SetPlayer%20Ref _asbp_my_player)
  (Utilities|FlowControl|Sequence
    (:then_0
      (Transformation|SetActorRotation (Math|Rotator|FindLookatRotation (Transformation|GetActorLocation) (Transformation|GetActorLocation (Variables|Default|GetPlayer%20Ref)))))
    (:then_1
      (if (Variables|Default|Getb_SpawnProjectile)
        (bind _returnvalue_2 (Game|SpawnActorfromClass "/Game/Characters/Player/BP_PlayerBullet.BP_PlayerBullet_C" (Transformation|GetWorldTransform (Variables|Default|GetProjectileSpawnLocation)) "Undefined" 0 0))
        (Variables|Default|SetProjectile%20Reference _returnvalue_2)
        (bind _outhit (Collision|LineTraceForObjects _returnvalue (+ _returnvalue (* (Math|Vector|GetForwardVector (Transformation|GetWorldRotation (Variables|Collision|GetCapsuleComponent))) 2e+05)) (Utilities|Array|MakeArray "ObjectTypeQuery1") false 0 "ForDuration" true "(R=1.000000,G=0.000000,B=0.000000,A=1.000000)" "(R=0.000000,G=1.000000,B=0.000000,A=1.000000)" 3.0))
        (Utilities|FlowControl|Delay 0.4)
        (Audio|PlaySound2D 0 1.0 1.0 0.0 0 0)
        (Effects|SpawnEmitteratLocation 0 (Transformation|GetWorldLocation _projectilespawnlocation_2) (Transformation|GetWorldRotation _projectilespawnlocation_2))
        (bind _outhit_2 (Collision|LineTraceForObjects (Transformation|GetWorldLocation (Variables|Default|GetProjectileSpawnLocation)) (.ImpactPoint (Collision|BreakHitResult _outhit)) (Utilities|Array|MakeArray "ObjectTypeQuery1" "ObjectTypeQuery2" "ObjectTypeQuery3" "ObjectTypeQuery5") false 0 "ForDuration" true "(R=1.000000,G=0.000000,B=0.000000,A=1.000000)" "(R=0.000000,G=1.000000,B=0.000000,A=1.000000)" 0.2))
        (Effects|SpawnEmitteratLocation 0 (.impactpoint _outhit_2))
        (Utilities|Casting|CastToBP_MyPlayer (.hitactor _outhit_2))
        (Utilities|FlowControl|Delay 1.0)
        (Actor|DestroyActor (Variables|Default|GetProjectile%20Reference))
        (Default|TakeDamage (Variables|Default|GetPlayer%20Ref) 1)
        (bind _asultimaki_game_mode (Utilities|Casting|CastToUltimakiGameMode (Game|GetGameMode)))
        (Default|UpdateHealth (Variables|/Game/Blueprints/GameModes/UltimakiGameMode.UltimakiGameMode_C|GetHUD _asultimaki_game_mode))
        (if (<= (Variables|/Game/Characters/Player/BP_MyPlayer.BP_MyPlayer_C|Geti_Health (Variables|Default|GetPlayer%20Ref)) 0)
          (Default|Death (Variables|Default|GetPlayer%20Ref))
          (else
            (Utilities|FlowControl|Delay 2.0)
            (Variables|Default|Setb_CanAttack true)))))))

(fn ConstructionScript)