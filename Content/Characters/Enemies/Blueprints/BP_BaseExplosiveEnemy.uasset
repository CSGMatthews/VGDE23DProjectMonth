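; Base explosive enemy that chases the player and detonates on reaching them, costing one health point.
; PawnSensing sighting of BP_MyPlayer starts AIMoveTo; on success, if attacking is allowed, the enemy destroys itself and spawns explosion effects at the player's location.
; It then refreshes the HUD through UltimakiGameMode and calls Death at zero health, otherwise starting an attack-cooldown delay despite the actor already being destroyed.
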(event OnSeePawn(PawnSensing)
  (params (Pawn :type Pawn%20Object%20Reference))
  ;[1 1 1] On Pawn Sence
  (bind _asbp_my_player (Utilities|Casting|CastToBP_MyPlayer Pawn))
  (bind _output_get (Variables|Default|SetPlayerReference _asbp_my_player))
  (AI|AIMoveTo self "0, 0, 0" _output_get 5.0 false
    (:OnSuccess
      ;;[1 1 1] If Player Is in Radius Spawn the Emitter and Sound
      (Variables|Default|Setb_IsPlayerInRadius true)
      (if (Variables|Default|Getb_CanAttack)
        (Variables|/Game/Characters/Player/BP_MyPlayer.BP_MyPlayer_C|Seti_PlayerHealth (Variables|Default|GetPlayerReference) (- (Variables|/Game/Characters/Player/BP_MyPlayer.BP_MyPlayer_C|Geti_PlayerHealth (Variables|Default|GetPlayerReference)) 1))
        (Actor|DestroyActor)
        (Effects|SpawnEmitteratLocation "/Game/StarterContent/Particles/P_Explosion.P_Explosion" (Transformation|GetActorLocation (Variables|Default|GetPlayerReference))) ; Spawn
        (Audio|PlaySoundatLocation "/Game/StarterContent/Audio/Explosion_Cue.Explosion_Cue" (Transformation|GetActorLocation (Variables|Default|GetPlayerReference)) "0, 0, 0" 1.0 1.0 0.0 0 0 0)
        (Variables|Default|Setb_CanAttack false)
        ;;[1 1 1] Update Health Hud And If they Still Have  Health Point Attack Again If They Down To One Health On This Next Hit Invoke the True For Death
        (bind _asultimaki_game_mode (Utilities|Casting|CastToUltimakiGameMode (Game|GetGameMode)))
        (Default|UpdateHealth (Variables|/Game/Blueprints/GameModes/UltimakiGameMode.UltimakiGameMode_C|GetHUD _asultimaki_game_mode))
        (if (<= (Variables|/Game/Characters/Player/BP_MyPlayer.BP_MyPlayer_C|Geti_PlayerHealth (Variables|Default|GetPlayerReference)) 0)
          (Default|Death (Variables|Default|GetPlayerReference))
          (else
            (Utilities|FlowControl|Delay 2.0)
            (Variables|Default|Setb_CanAttack true)))))))

(fn ConstructionScript)