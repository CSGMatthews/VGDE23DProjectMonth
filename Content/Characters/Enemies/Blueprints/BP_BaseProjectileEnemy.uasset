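; Base projectile enemy that turns to face the player and shoots when its PawnSensing component sees them.
; Each sighting of BP_MyPlayer stores the player reference and snaps the actor's rotation toward them.
; If the fire flag is set, it spawns BP_EnemyBullet at ProjectileSpawnLocation with a sound and emitter effect, then blocks firing until a cooldown delay ends.
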(event OnSeePawn(PawnSensing)
  (params (Pawn :type Pawn%20Object%20Reference))
  (bind _projectilespawnlocation (Variables|Default|GetProjectileSpawnLocation))
  ;[1 1 1] On Pawn Sence start firing and dealing damage
  (bind _asbp_my_player (Utilities|Casting|CastToBP_MyPlayer Pawn))
  (Variables|Default|SetPlayer%20Ref _asbp_my_player)
  (Utilities|FlowControl|Sequence
    (:then_0
      (Transformation|SetActorRotation (Math|Rotator|FindLookatRotation (Transformation|GetActorLocation) (Transformation|GetActorLocation (Variables|Default|GetPlayer%20Ref)))))
    (:then_1
      (if (Variables|Default|Getb_SpawnProjectile)
        (bind _returnvalue (Game|SpawnActorfromClass "/Game/Characters/Enemies/Weapons/BP_EnemyBullet.BP_EnemyBullet_C" (Transformation|GetWorldTransform (Variables|Default|GetProjectileSpawnLocation)) "Undefined" 0 0))
        (Variables|Default|SetProjectile%20Reference _returnvalue)
        (Variables|Default|Setb_SpawnProjectile false)
        (Audio|PlaySound2D "/Game/Assets/Audio/SFX/vgmenuselect_Cue.vgmenuselect_Cue" 1.0 1.0 0.0 0 0)
        (Effects|SpawnEmitteratLocation 0 (Transformation|GetWorldLocation _projectilespawnlocation) (Transformation|GetWorldRotation _projectilespawnlocation))
        (Utilities|FlowControl|Delay 5.0)
        (Variables|Default|Setb_SpawnProjectile true)))))

(fn ConstructionScript)