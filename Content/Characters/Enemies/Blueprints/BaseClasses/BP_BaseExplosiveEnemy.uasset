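; Base Blueprint for a suicide-style enemy that chases the player and destroys itself on contact.
; PawnSensing triggers an AI MoveTo toward the seen player, and a one-time box overlap applies damage through the Ultimaki game instance before destroying the actor.
; TakeDamage reduces health, playing a sound and montage on non-lethal hits, or a sound and emitter on death, followed by delayed destruction and a health pickup spawn.
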(event OnSeePawn(PawnSensing)
  (params (Pawn :type Pawn%20Object%20Reference))
  ;[1 1 1] On Pawn Sence
  (bind _asbp_my_player (Utilities|Casting|CastToBP_MyPlayer Pawn))
  (bind _output_get (Variables|Default|SetPlayerReference _asbp_my_player))
  (AI|AIMoveTo self "0, 0, 0" _output_get 5.0 false))

(event OnComponentBeginOverlap(Box)
  (params (OverlappedComponent :type Primitive%20Component%20Object%20Reference) (OtherActor :type Actor%20Object%20Reference) (OtherComp :type Primitive%20Component%20Object%20Reference) (OtherBodyIndex :type Integer) (bFromSweep :type Boolean) (SweepResult :type Hit%20Result%20Structure%20%28by%20ref%29))
  (Utilities|Casting|CastToBP_MyPlayer OtherActor)
  (Utilities|FlowControl|DoOnce false
    (:Completed
      (bind _asultimaki_game_instance (Utilities|Casting|CastToUltimaki_GameInstance (Game|GetGameInstance)))
      (Default|TakeDamage _asultimaki_game_instance 1)
      (Actor|DestroyActor))))

(event Custom|TakeDamage
  (params (Damage :type Integer))
  ;[1 1 1] TakeDamage
  (bind _output_get (Variables|Default|Seti_EnemyHealth (- (Variables|Default|Geti_EnemyHealth) Damage)))
  (if (<= _output_get 0)
    (Audio|PlaySound2D 0 1.0 1.0 0.0 0 0)
    (Effects|SpawnEmitteratLocation 0 "0, 0, 0")
    (Utilities|FlowControl|Delay 0.2)
    (Actor|DestroyActor)
    (Game|SpawnActorfromClass "/Game/Blueprints/Actors/PowerUps/BP_Health_POW.BP_Health_POW_C" (Math|Transform|MakeTransform (Transformation|GetActorLocation) "0, 0, 0" "1,1,1") "AlwaysSpawn" 0 0)
    (else
      (Audio|PlaySound2D 0 1.0 1.0 0.0 0 0)
      (Animation|Montage|PlayMontage (Variables|Character|GetMesh) 0))))

(fn ConstructionScript)