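; Enemy spawner actor that periodically spawns at its own location and rotation.
; BeginPlay starts a looping timer whose Spawn event randomly selects between the tiny chef enemy class and a second, blank option.
; Separate AttemptToSpawn and SpawnItem functions place a random power-up only when no current item exists, but the event graph never calls them.
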(event Custom|Spawn
  (Game|SpawnActorfromClass (Utilities|Select :Index (Math|Random|RandomIntegerinRange 0 1) :Option%200 "/Game/Blueprints/Characters/Enemies/Blueprints/TinyChef/BP_TinyChefEnemy_.BP_TinyChefEnemy__C" :Option%201 0) (Math|Transform|MakeTransform (Transformation|GetActorLocation) (Transformation|GetActorRotation)) "Undefined" 0 0))

(event EventBeginPlay
  (Utilities|Time|SetTimerbyEvent (delegate Custom|Spawn) 5.0 true))

(fn ConstructionScript)

(fn AttempttoSpawn
  (Utilities|IsValid (Variables|Default|GetCurrentItem)
    (:Is%20Valid
      (Development|PrintString "ItemAlreadySpaw\\ned"))
    (:Is%20Not%20Valid
      (CallFunction|SpawnItem))))

(fn SpawnItem
  (bind _returnvalue (Game|SpawnActorfromClass (Utilities|Array|Get(acopy) (Variables|Default|Getbp_PowerUpsToSpawn) (Math|Random|RandomIntegerinRange 0 (- (Utilities|Array|Length (Variables|Default|Getbp_PowerUpsToSpawn)) 1))) (Math|Transform|MakeTransform (Transformation|GetActorLocation) (Transformation|GetActorRotation)) "AlwaysSpawn" self 0))
  (Variables|Default|SetCurrentItem _returnvalue))