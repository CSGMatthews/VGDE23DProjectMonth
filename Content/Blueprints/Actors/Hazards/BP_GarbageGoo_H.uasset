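; BP_GarbageGoo_H is a garbage goo hazard actor that damages the player over time while they stay inside its HazardArea.
; Begin overlap removes one health from BP_MyPlayer, refreshes the health display through the UltimakiGameMode HUD, and repeats on a half-second Delay loop while an in-radius flag is set.
; The loop calls Death on the player character once health runs out, and end overlap clears the flag to stop further damage.
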(event OnComponentBeginOverlap(HazardArea)
  (params (OverlappedComponent :type Primitive%20Component%20Object%20Reference) (OtherActor :type Actor%20Object%20Reference) (OtherComp :type Primitive%20Component%20Object%20Reference) (OtherBodyIndex :type Integer) (bFromSweep :type Boolean) (SweepResult :type Hit%20Result%20Structure%20%28by%20ref%29))
  ;[1 1 1] Player is in radius so keep dealing damage
  (bind _asbp_my_player (Utilities|Casting|CastToBP_MyPlayer OtherActor))
  (Variables|Default|Setb_PlayerInRadius true)
  (bind _output_get (Variables|/Game/Characters/Player/BP_MyPlayer.BP_MyPlayer_C|Seti_Health _asbp_my_player (- (Variables|/Game/Characters/Player/BP_MyPlayer.BP_MyPlayer_C|Geti_Health _asbp_my_player) 1) :!label _label))
  (bind _asultimaki_game_mode (Utilities|Casting|CastToUltimakiGameMode (Game|GetGameMode)))
  (Default|UpdateHealth (Variables|/Game/Blueprints/GameModes/UltimakiGameMode.UltimakiGameMode_C|GetHUD _asultimaki_game_mode))
  (if (<= _output_get 0)
    (bind _asbp_my_player_2 (Utilities|Casting|CastToBP_MyPlayer (Game|GetPlayerCharacter 0)))
    (Default|Death _asbp_my_player_2)
    (else
      (Utilities|FlowControl|Delay 0.5)
      (if (Variables|Default|Getb_PlayerInRadius)
        (goto _label)))))

(event OnComponentEndOverlap(HazardArea)
  (params (OverlappedComponent :type Primitive%20Component%20Object%20Reference) (OtherActor :type Actor%20Object%20Reference) (OtherComp :type Primitive%20Component%20Object%20Reference) (OtherBodyIndex :type Integer))
  ;[1 1 1] If out of radius stop dealing damage
  (Utilities|Casting|CastToBP_MyPlayer OtherActor)
  (Variables|Default|Setb_PlayerInRadius false))

(fn ConstructionScript)