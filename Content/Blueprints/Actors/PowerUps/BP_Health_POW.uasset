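; Health power-up pickup that adds one point to the player's health, stored in Ultimaki_GameInstance, while it is below five.
; A box overlap fires once without filtering the overlapping actor; at full health it does nothing, leaving the pickup spent but present.
; On success it shows a widget, refreshes the HUD, plays a sound and attaches a brief aura to the player, then destroys itself.
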(event OnComponentBeginOverlap(Box_0)
  (params (OverlappedComponent :type Primitive%20Component%20Object%20Reference) (OtherActor :type Actor%20Object%20Reference) (OtherComp :type Primitive%20Component%20Object%20Reference) (OtherBodyIndex :type Integer) (bFromSweep :type Boolean) (SweepResult :type Hit%20Result%20Structure%20%28by%20ref%29))
  (bind _asultimaki_game_instance (Utilities|Casting|CastToUltimaki_GameInstance (Game|GetGameInstance)))
  (bind _output_get (Variables|Default|SetGameInstanceReference _asultimaki_game_instance))
  (Utilities|FlowControl|DoOnce false
    (:Completed
      (if (< (Variables|/Game/Blueprints/GameModes/Ultimaki_GameInstance.Ultimaki_GameInstance_C|Geti_PlayerHealth _asultimaki_game_instance) 5)
        (bind _returnvalue (UserInterface|CreateWidget "/Game/Blueprints/Widgets/PickUps/WB_Health_POW.WB_Health_POW_C"))
        (UserInterface|Viewport|AddtoViewport _returnvalue 0)
        (Variables|/Game/Blueprints/GameModes/Ultimaki_GameInstance.Ultimaki_GameInstance_C|Seti_PlayerHealth _output_get (+ (Variables|/Game/Blueprints/GameModes/Ultimaki_GameInstance.Ultimaki_GameInstance_C|Geti_PlayerHealth _asultimaki_game_instance) 1))
        (Default|UpdateHealth (Variables|/Game/Blueprints/GameModes/Ultimaki_GameInstance.Ultimaki_GameInstance_C|Getbp_HUDReference _asultimaki_game_instance))
        (bind _asbp_my_player (Utilities|Casting|CastToBP_MyPlayer (Game|GetPlayerCharacter 0)))
        (Audio|PlaySound2D "/Game/Assets/Audio/SFX/Powerups/Powerup__001.Powerup__001" 1.0 1.0 0.0 0 0)
        (bind _returnvalue_2 (Effects|SpawnEmitterAttached "/Game/Assets/Particles/FX_Combat/P_AuraCircle_LeachTarget.P_AuraCircle_LeachTarget" (Variables|/Game/Blueprints/Characters/Player/BP_MyPlayer.BP_MyPlayer_C|GetHurt _asbp_my_player) "None" "0, 0, 0" "0, 0, 0" "1.000000,1.000000,1.000000" "SnapToTargetIncludingScale"))
        (Utilities|FlowControl|Delay 2.0)
        (Components|DestroyComponent _returnvalue_2)
        (Actor|DestroyActor)))))

(event EventBeginPlay)

(event Collision|EventActorBeginOverlap
  (params (OtherActor :type Actor%20Object%20Reference)))

(event EventTick
  (params (DeltaSeconds :type Float%20%28single-precision%29)))

(fn ConstructionScript)