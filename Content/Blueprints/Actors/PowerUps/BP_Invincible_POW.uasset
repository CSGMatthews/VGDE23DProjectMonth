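; BP_Invincible_POW is an invincibility power-up actor that acts on BP_MyPlayer when it overlaps it.
; A DoOnce lets the first pickup attach a particle effect to the player's body, play a sound and start the Duration timeline.
; Each timeline update writes the truncated HealthBoost track to the player's IPlayerHealth.
; The first update also starts a six-second Delay that destroys the actor.
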(event Collision|EventActorBeginOverlap
  (params (OtherActor :type Actor%20Object%20Reference))
  ;[1 1 1] Once pick up set the duration of the powerup
  (Development|PrintString "Invincible")
  (bind _asbp_my_player (Utilities|Casting|CastToBP_MyPlayer OtherActor))
  (Variables|Default|SetPlayerReference _asbp_my_player)
  (Utilities|FlowControl|DoOnce false
    (:Completed
      (Effects|SpawnEmitterAttached "/Game/Assets/Particles/FX_Ability/Heal/P_HealthPotion_Pickup_01.P_HealthPotion_Pickup_01" (Variables|/Game/Characters/Player/BP_MyPlayer.BP_MyPlayer_C|GetBody _asbp_my_player) "None" (Transformation|GetActorLocation _asbp_my_player) (Transformation|GetActorRotation _asbp_my_player))
      (Audio|PlaySound2D "/Game/Assets/Audio/SFX/Powerups/Powerup__003.Powerup__003" 1.0 1.0 0.0 0 0)
      (bind _healthboost (Timeline|Duration Play)
        (:Update
          (Variables|/Game/Characters/Player/BP_MyPlayer.BP_MyPlayer_C|Seti_PlayerHealth (Variables|Default|GetPlayerReference) (Math|Float|Truncate _healthboost))
          (Utilities|FlowControl|Delay 6.0)
          (Actor|DestroyActor))))))

(fn ConstructionScript)