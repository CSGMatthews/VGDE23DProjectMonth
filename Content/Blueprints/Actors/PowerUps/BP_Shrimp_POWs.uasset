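; BP_Shrimp_POWs is a power-up pickup that changes the player's jump strength.
; When BP_MyPlayer overlaps it, a DoOnce gate attaches a spark emitter to the player's body, plays a sound and starts a timeline.
; The timeline's JumpBoost track drives the character's JumpZVelocity on each update.
; A Delay on that update path destroys the pickup about six seconds after the timeline starts.
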(event Collision|EventActorBeginOverlap
  (params (OtherActor :type Actor%20Object%20Reference))
  ;[1 1 1] Once pick up set the duration of the powerup
  (bind _asbp_my_player (Utilities|Casting|CastToBP_MyPlayer OtherActor))
  (Variables|Default|SetPlayerRef _asbp_my_player)
  (Utilities|FlowControl|DoOnce false
    (:Completed
      (Effects|SpawnEmitterAttached "/Game/StarterContent/Particles/P_Sparks.P_Sparks" (Variables|/Game/Characters/Player/BP_MyPlayer.BP_MyPlayer_C|GetBody _asbp_my_player) "None" (Transformation|GetActorLocation _asbp_my_player) (Transformation|GetActorRotation _asbp_my_player))
      (Audio|PlaySound2D "/Game/StarterContent/Audio/Explosion01.Explosion01" 1.0 1.0 0.0 0 0)
      (bind _jumpboost (Timeline|Timeline_0 Play)
        (:Update
          (Variables|/Script/Engine.CharacterMovementComponent|SetJumpZVelocity (Variables|/Script/Engine.Character|GetCharacterMovement (Variables|Default|GetPlayerRef)) _jumpboost)
          (Utilities|FlowControl|Delay 6.0)
          (Actor|DestroyActor))))))

(fn ConstructionScript)