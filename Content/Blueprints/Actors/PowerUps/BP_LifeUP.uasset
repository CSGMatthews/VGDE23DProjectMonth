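; BP_LifeUP is an extra-life pickup that grants the player one additional life on touch.
; Overlapping its Sphere with a BP_MyPlayer increments IPlayerLives on Ultimaki_GameInstance, so the life count is stored in the game instance.
; It then calls Collected, which clears the static mesh, destroys the collision sphere and sets BIsCollected, leaving the actor itself in the level.
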(event OnComponentBeginOverlap(Sphere)
  (params (OverlappedComponent :type Primitive%20Component%20Object%20Reference) (OtherActor :type Actor%20Object%20Reference) (OtherComp :type Primitive%20Component%20Object%20Reference) (OtherBodyIndex :type Integer) (bFromSweep :type Boolean) (SweepResult :type Hit%20Result%20Structure%20%28by%20ref%29))
  (Utilities|Casting|CastToBP_MyPlayer OtherActor)
  (bind _asultimaki_game_instance (Utilities|Casting|CastToUltimaki_GameInstance (Game|GetGameInstance)))
  (Variables|/Game/Blueprints/GameModes/Ultimaki_GameInstance.Ultimaki_GameInstance_C|Seti_PlayerLives _asultimaki_game_instance (+ (Variables|/Game/Blueprints/GameModes/Ultimaki_GameInstance.Ultimaki_GameInstance_C|Geti_PlayerLives _asultimaki_game_instance) 1))
  (CallFunction|Collected))

(event Custom|Collected
  ;[1 1 1] Collected
  (Components|StaticMesh|SetStaticMesh (Variables|Default|GetStaticMesh) 0)
  (Components|DestroyComponent (Variables|Default|GetSphere))
  (Variables|Default|Setb_IsCollected? true))

(event EventBeginPlay)

(event Collision|EventActorBeginOverlap
  (params (OtherActor :type Actor%20Object%20Reference)))

(event EventTick
  (params (DeltaSeconds :type Float%20%28single-precision%29)))

(fn ConstructionScript)