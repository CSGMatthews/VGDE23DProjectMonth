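; Rice power-up actor that changes the player's walk speed when BP_MyPlayer overlaps it.
; The first pickup attaches a spark emitter to the player's body, plays a sound and starts the Duration timeline.
; The timeline's SpeedBoost track drives MaxWalkSpeed on each update, which also feeds a delay that destroys the actor a few seconds later.
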(event Collision|EventActorBeginOverlap
  (params (OtherActor :type Actor%20Object%20Reference))
  ;[1 1 1] Once pick up set the duration of the powerup
  (bind _asbp_my_player (Utilities|Casting|CastToBP_MyPlayer OtherActor))
  (bind _output_get (Variables|Default|SetPlayerReference _asbp_my_player))
  (Utilities|FlowControl|DoOnce false
    (:Completed
      (Effects|SpawnEmitterAttached "/Game/StarterContent/Particles/P_Sparks.P_Sparks" (Variables|/Game/Characters/Player/BP_MyPlayer.BP_MyPlayer_C|GetBody _output_get) "None")
      (Audio|PlaySound2D "/Game/Assets/Audio/SFX/Powerups/Powerup__003.Powerup__003" 1.0 1.0 0.0 0 0)
      (bind _speedboost (Timeline|Duration Play)
        (:Update
          (Variables|/Script/Engine.CharacterMovementComponent|SetMaxWalkSpeed (Variables|/Script/Engine.Character|GetCharacterMovement (Variables|Default|GetPlayerReference)) _speedboost)
          (Utilities|FlowControl|Delay 6.0)
          (Actor|DestroyActor))))))

(fn ConstructionScript)