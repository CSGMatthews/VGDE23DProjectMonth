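; BP_Crab_POW is a health power-up actor that the player collects by touching it.
; When its Box overlaps a BP_MyPlayer, it adds one to the player's health with no cap check, plays a sound and attaches an absorb particle effect to the player's body.
; It then refreshes the health HUD through UltimakiGameMode and destroys itself, which only happens if that game mode cast succeeds.
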(event OnComponentBeginOverlap(Box)
  (params (OverlappedComponent :type Primitive%20Component%20Object%20Reference) (OtherActor :type Actor%20Object%20Reference) (OtherComp :type Primitive%20Component%20Object%20Reference) (OtherBodyIndex :type Integer) (bFromSweep :type Boolean) (SweepResult :type Hit%20Result%20Structure%20%28by%20ref%29))
  (bind _asbp_my_player (Utilities|Casting|CastToBP_MyPlayer OtherActor))
  (bind _output_get (Variables|Default|SetPlayerRef _asbp_my_player))
  (Variables|/Game/Characters/Player/BP_MyPlayer.BP_MyPlayer_C|Seti_PlayerHealth _output_get (+ (Variables|/Game/Characters/Player/BP_MyPlayer.BP_MyPlayer_C|Geti_PlayerHealth _asbp_my_player) 1))
  (Audio|PlaySound2D "/Game/Assets/Audio/SFX/Powerups/Powerup__001.Powerup__001" 1.0 1.0 0.0 0 0)
  (Effects|SpawnEmitterAttached "/Game/Assets/Particles/FX_Combat/P_Health_Absorb_01.P_Health_Absorb_01" (Variables|/Game/Characters/Player/BP_MyPlayer.BP_MyPlayer_C|GetBody (Variables|Default|GetPlayerRef)) "None")
  (bind _asultimaki_game_mode (Utilities|Casting|CastToUltimakiGameMode (Game|GetGameMode)))
  (Default|UpdateHealth (Variables|/Game/Blueprints/GameModes/UltimakiGameMode.UltimakiGameMode_C|GetHUD _asultimaki_game_mode))
  (Actor|DestroyActor))

(event EventBeginPlay)

(event Collision|EventActorBeginOverlap
  (params (OtherActor :type Actor%20Object%20Reference)))

(event EventTick
  (params (DeltaSeconds :type Float%20%28single-precision%29)))

(fn ConstructionScript)