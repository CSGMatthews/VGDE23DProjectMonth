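; BP_Speed_POW is a speed power-up pickup that changes the player's walk speed through a timeline.
; On box overlap with BP_MyPlayer, a DoOnce attaches a particle effect to the player's InvinciblePowerUp component, plays a sound and starts the Duration timeline.
; The timeline's SpeedBoost track drives MaxWalkSpeed, and its finish plays a power-off sound.
; A delay triggered from the timeline's update destroys the actor.
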(event OnComponentBeginOverlap(Box)
  (params (OverlappedComponent :type Primitive%20Component%20Object%20Reference) (OtherActor :type Actor%20Object%20Reference) (OtherComp :type Primitive%20Component%20Object%20Reference) (OtherBodyIndex :type Integer) (bFromSweep :type Boolean) (SweepResult :type Hit%20Result%20Structure%20%28by%20ref%29))
  ;[1 1 1] Once pick up set the duration of the powerup
  (bind _asbp_my_player (Utilities|Casting|CastToBP_MyPlayer OtherActor))
  (Variables|Default|SetPlayerReference _asbp_my_player)
  (Utilities|FlowControl|DoOnce false
    (:Completed
      (Effects|SpawnEmitterAttached "/Game/Assets/Particles/FX_Combat/WeaponCombo/P_ComboFinish_Tap_02.P_ComboFinish_Tap_02" (Variables|/Game/Blueprints/Characters/Player/BP_MyPlayer.BP_MyPlayer_C|GetInvinciblePowerUp _asbp_my_player) "None")
      (Audio|PlaySound2D "/Game/Assets/Audio/SFX/Powerups/Powerup__003.Powerup__003" 1.0 1.0 0.0 0 0)
      (bind _speedboost (Timeline|Duration Play)
        (:Update
          (Variables|/Script/Engine.CharacterMovementComponent|SetMaxWalkSpeed (Variables|/Script/Engine.Character|GetCharacterMovement (Variables|Default|GetPlayerReference)) _speedboost)
          (Utilities|FlowControl|Delay 6.0)
          (Actor|DestroyActor))
        (:Finished
          (Audio|PlaySound2D "/Game/Assets/Audio/SFX/MachinePowerOff.MachinePowerOff" 1.0 1.0 0.0 0 0))))))

(fn ConstructionScript)