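; BP_SignPost is a signpost actor that shows its own text in a dialogue box when interacted with.
; Its Interact event works as a toggle: it removes and clears the stored WB_Dialogue widget if valid, otherwise creates one for player controller 0.
; The new widget is stored, added to the viewport and given the sign's MyText as its dialogue text.
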(event EventInteract
  (Utilities|IsValid (Variables|Default|GetDialogueReference)
    (:Is%20Valid
      (Widget|RemovefromParent (Variables|Default|GetDialogueReference))
      (Variables|Default|SetDialogueReference 0))
    (:Is%20Not%20Valid
      (bind _returnvalue (UserInterface|CreateWidget "/Game/Blueprints/Widgets/Dialogue/WB_Dialogue.WB_Dialogue_C" (Game|GetPlayerController 0)))
      (bind _output_get (Variables|Default|SetDialogueReference _returnvalue))
      (UserInterface|Viewport|AddtoViewport _output_get 0)
      (Variables|/Game/Blueprints/Widgets/Dialogue/WB_Dialogue.WB_Dialogue_C|SetDialogueText (Variables|Default|GetDialogueReference) (Variables|Default|GetMyText)))))

(fn ConstructionScript)