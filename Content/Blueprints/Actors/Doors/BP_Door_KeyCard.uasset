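; Key card door that the player opens with E and that slides back when they leave its box trigger.
; On overlap it checks the player's key card array at the door's key value index, enabling input and playing a delayed sound on a match.
; E plays a door sound and the DoorAnimation timeline that moves the mesh; end overlap reverses it.
; Input is never disabled again after being granted.
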(event OnComponentBeginOverlap(Box)
  (params (OverlappedComponent :type Primitive%20Component%20Object%20Reference) (OtherActor :type Actor%20Object%20Reference) (OtherComp :type Primitive%20Component%20Object%20Reference) (OtherBodyIndex :type Integer) (bFromSweep :type Boolean) (SweepResult :type Hit%20Result%20Structure%20%28by%20ref%29))
  (bind _asbp_my_player (Utilities|Casting|CastToBP_MyPlayer OtherActor))
  (for (_array_element _array_index) (Variables|/Game/Characters/Player/BP_MyPlayer.BP_MyPlayer_C|Getb_KeyCards _asbp_my_player)
    (if (and _array_element (== _array_index (Variables|Default|Geti_KeyCardValue)))
      (Input|EnableInput (Game|GetPlayerController 0))
      (Utilities|FlowControl|Delay 2.0)
      (Audio|PlaySound2D "/Game/Assets/Audio/SFX/vgmenuselect.vgmenuselect" 1.0 1.0 0.0 0 0))))

(event OnComponentEndOverlap(Box)
  (params (OverlappedComponent :type Primitive%20Component%20Object%20Reference) (OtherActor :type Actor%20Object%20Reference) (OtherComp :type Primitive%20Component%20Object%20Reference) (OtherBodyIndex :type Integer))
  (Utilities|Casting|CastToBP_MyPlayer OtherActor)
  (bind _doorslide (Timeline|DoorAnimation Reverse)
    (:Update
      (Transformation|SetRelativeLocation (Variables|Default|GetProxDoorMesh) _doorslide false false))))

(event Input|KeyboardEvents|E
  (params (Key :type Key%20Structure :default "None"))
  (:Pressed
    (Audio|PlaySound2D "/Game/Assets/Audio/SFX/Door/doorClose_1.doorClose_1" 1.0 1.0 0.0 0 0)
    (bind _doorslide (Timeline|DoorAnimation Play)
      (:Update
        (Transformation|SetRelativeLocation (Variables|Default|GetProxDoorMesh) _doorslide false false)))))

(fn ConstructionScript)