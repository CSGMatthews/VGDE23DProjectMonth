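; Pressure plate actor that opens and closes a pressure door when a push block moves on or off it.
; On overlap it lowers its body, searches all pressure door actors for one whose DoorID matches the plate's ID, and opens it.
; When the block leaves, it waits briefly, moves the body back, repeats the search and closes that door.
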(event Collision|EventActorBeginOverlap
  (params (OtherActor :type Actor%20Object%20Reference))
  ;[1 1 1] On Begin Overlap open the door
  (Utilities|Casting|CastToBP_PushBlock OtherActor)
  (Components|MoveComponentTo (Variables|Default|GetBody) "0, 0,-40.000000" "0, 0, 0" false false 0.2 false)
  (bind _outactors (Actor|GetAllActorsOfClass "/Game/Blueprints/Actors/Doors/Door_Pressure_BP.Door_Pressure_BP_C"))
  (for _array_element _outactors
    (if (== (Variables|/Game/Blueprints/Actors/Doors/Door_Pressure_BP.Door_Pressure_BP_C|GetDoorID _array_element) (Variables|Default|GetPressurePlateID))
      (Variables|Default|SetDoor _array_element)))
  (Utilities|IsValid (Variables|Default|GetDoor)
    (:Is%20Valid
      (Default|Open (Variables|Default|GetDoor)))))

(event Collision|EventActorEndOverlap
  (params (OtherActor :type Actor%20Object%20Reference))
  ;[1 1 1] On End Overlap close the door
  (Utilities|Casting|CastToBP_PushBlock OtherActor)
  (Utilities|FlowControl|Delay 1.0)
  (Components|MoveComponentTo (Variables|Default|GetBody) "0, 0, 0" "0, 0, 0" false false 0.2 false)
  (bind _outactors (Actor|GetAllActorsOfClass "/Game/Blueprints/Actors/Doors/Door_Pressure_BP.Door_Pressure_BP_C"))
  (for _array_element _outactors
    (if (== (Variables|/Game/Blueprints/Actors/Doors/Door_Pressure_BP.Door_Pressure_BP_C|GetDoorID _array_element) (Variables|Default|GetPressurePlateID))
      (Variables|Default|SetDoor _array_element)))
  (Utilities|IsValid (Variables|Default|GetDoor)
    (:Is%20Valid
      (Default|Close (Variables|Default|GetDoor)))))

(fn ConstructionScript)