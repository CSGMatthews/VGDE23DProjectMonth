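; Restaurant sliding door that stays locked until its linked BPSwitch is pressed, with a LockLight showing red when locked and green when unlocked.
; The construction script sets the initial light color, and the switch's pressed event clears the lock and turns the light green.
; The overlap box enables input and shows an interact prompt; Interact plays a locked sound or opens the door via a timeline, which reverses when the player leaves.
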(event OnComponentBeginOverlap(Box)
  (params (OverlappedComponent :type Primitive%20Component%20Object%20Reference) (OtherActor :type Actor%20Object%20Reference) (OtherComp :type Primitive%20Component%20Object%20Reference) (OtherBodyIndex :type Integer) (bFromSweep :type Boolean) (SweepResult :type Hit%20Result%20Structure%20%28by%20ref%29))
  ;[1 1 1] On begin overlap if the door is unlocked play the sound when you open it
  (bind _asbp_my_player (Utilities|Casting|CastToBP_MyPlayer OtherActor))
  (Input|EnableInput (Game|GetPlayerController 0))
  (Variables|/Game/Blueprints/Characters/Player/BP_MyPlayer.BP_MyPlayer_C|SetGameMessage _asbp_my_player "Press F To Interact"))

(event OnComponentEndOverlap(Box)
  (params (OverlappedComponent :type Primitive%20Component%20Object%20Reference) (OtherActor :type Actor%20Object%20Reference) (OtherComp :type Primitive%20Component%20Object%20Reference) (OtherBodyIndex :type Integer))
  ;[1 1 1] On begin overlap if the door is unlocked play the sound when you open it
  (bind _asbp_my_player (Utilities|Casting|CastToBP_MyPlayer OtherActor))
  (Input|DisableInput (Game|GetPlayerController 0))
  (Variables|/Game/Blueprints/Characters/Player/BP_MyPlayer.BP_MyPlayer_C|SetGameMessage _asbp_my_player "")
  (bind _doorslide (Timeline|DoorAnimation Reverse)
    (:Update
      (Transformation|SetRelativeLocation (Variables|Default|GetProxDoorMesh) _doorslide false false))))

(event Custom|UnlockDoor
  (params (Switch :type Trigger%20Switch%20BP%20Object%20Reference))
  (bind _locklight (Variables|Default|GetLockLight))
  ;[1 1 1] Sets the Color
  (if (== Switch (Variables|Default|GetBP_Switch))
    (bind _output_get (Variables|Default|Setb_IsLocked false))
    (if _output_get
      (Rendering|Components|Light|SetLightColor _locklight "(R=1.000000,G=0.015278,B=0.000000,A=1.000000)" true)
      (else
        (Rendering|Components|Light|SetLightColor _locklight "(R=0.000000,G=1.000000,B=0.191391,A=1.000000)" true)))))

(event EventBeginPlay
  ;[1 1 1] Sets the Color
  (EventDispatchers|BindEventtoSwitchPressed (Variables|Default|GetBP_Switch) (delegate Custom|UnlockDoor)))

(event Input|ActionEvents|InputActionInteract
  (params (Key :type Key%20Structure))
  ;[1 1 1] On begin overlap if the door is unlocked play the sound when you open it
  (:Pressed
    (if (Variables|Default|Getb_IsLocked)
      (Audio|PlaySound2D "/Game/Assets/Audio/SFX/Door/creak3.creak3" 1.0 1.0 0.0 0 0)
      (else
        (Audio|PlaySound2D "/Game/Assets/Audio/Kitchen_15.Kitchen_15" 1.0 1.0 1.0 0 0)
        (bind _doorslide (Timeline|DoorAnimation Play)
          (:Update
            (Transformation|SetRelativeLocation (Variables|Default|GetProxDoorMesh) _doorslide false false)))))))

(fn ConstructionScript
  (bind _locklight (Variables|Default|GetLockLight))
  (if (Variables|Default|Getb_IsLocked)
    (Rendering|Components|Light|SetLightColor _locklight "(R=1.000000,G=0.015278,B=0.000000,A=1.000000)" true)
    (else
      (Rendering|Components|Light|SetLightColor _locklight "(R=0.000000,G=1.000000,B=0.191391,A=1.000000)" true))))