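; Sliding door actor that the player opens with the Interact input while standing inside its box trigger.
; Overlap enables input on the actor and sets an interact prompt in BP_MyPlayer's GameMessage.
; Interacting plays a menu-select sound and the DoorAnimation timeline, which drives the door mesh's relative location.
; Leaving the box disables input, clears the prompt and reverses the timeline to slide the door back.
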(event OnComponentBeginOverlap(Box)
  (params (OverlappedComponent :type Primitive%20Component%20Object%20Reference) (OtherActor :type Actor%20Object%20Reference) (OtherComp :type Primitive%20Component%20Object%20Reference) (OtherBodyIndex :type Integer) (bFromSweep :type Boolean) (SweepResult :type Hit%20Result%20Structure%20%28by%20ref%29))
  (bind _asbp_my_player (Utilities|Casting|CastToBP_MyPlayer OtherActor))
  (Input|EnableInput (Game|GetPlayerController 0))
  (Variables|/Game/Characters/Player/BP_MyPlayer.BP_MyPlayer_C|SetGameMessage _asbp_my_player "Press F to Interact"))

(event OnComponentEndOverlap(Box)
  (params (OverlappedComponent :type Primitive%20Component%20Object%20Reference) (OtherActor :type Actor%20Object%20Reference) (OtherComp :type Primitive%20Component%20Object%20Reference) (OtherBodyIndex :type Integer))
  (bind _asbp_my_player (Utilities|Casting|CastToBP_MyPlayer OtherActor))
  (Input|DisableInput (Game|GetPlayerController 0))
  (Variables|/Game/Characters/Player/BP_MyPlayer.BP_MyPlayer_C|SetGameMessage _asbp_my_player "")
  (bind _doorslide (Timeline|DoorAnimation Reverse)
    (:Update
      (Transformation|SetRelativeLocation (Variables|Default|GetProxDoorMesh) _doorslide false false))))

(event Input|ActionEvents|InputActionInteract
  (params (Key :type Key%20Structure))
  (:Pressed
    (Audio|PlaySound2D "/Game/Assets/Audio/SFX/vgmenuselect.vgmenuselect" 1.0 1.0 0.0 0 0)
    (bind _doorslide (Timeline|DoorAnimation Play)
      (:Update
        (Transformation|SetRelativeLocation (Variables|Default|GetProxDoorMesh) _doorslide false false)))))

(fn ConstructionScript)