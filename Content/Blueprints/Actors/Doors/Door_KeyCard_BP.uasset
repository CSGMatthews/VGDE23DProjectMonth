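; Keycard-locked sliding door that the player opens with the Interact input while inside its trigger box.
; On overlap it checks the game instance's keycard array at its own index, then enables input with a prompt or shows a missing-keycard message.
; Interact plays a creak and the slide timeline; the player leaving clears the message, disables input and reverses the slide.
; A push-block overlap jumps into the same keycard check, reusing previously stored references.
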(event OnComponentBeginOverlap(Box)
  (params (OverlappedComponent :type Primitive%20Component%20Object%20Reference) (OtherActor :type Actor%20Object%20Reference) (OtherComp :type Primitive%20Component%20Object%20Reference) (OtherBodyIndex :type Integer) (bFromSweep :type Boolean) (SweepResult :type Hit%20Result%20Structure%20%28by%20ref%29))
  ;[1 1 1] On Begin overlap if we have the key card print the message and it will open on key press and play a sound
  (bind _asbp_my_player (Utilities|Casting|CastToBP_MyPlayer OtherActor)
    (:then
      (Variables|Default|SetPlayerRef _asbp_my_player)
      (bind _asultimaki_game_instance (Utilities|Casting|CastToUltimaki_GameInstance (Game|GetGameInstance))))
    (:CastFailed
      (Utilities|Casting|CastToBP_PushBlock OtherActor)))
  (if (Utilities|Array|Get(acopy) (Variables|/Game/Blueprints/GameModes/Ultimaki_GameInstance.Ultimaki_GameInstance_C|Getb_KeyCards? _asultimaki_game_instance) (Variables|Default|Geti_KeyCardValue))
    (Input|EnableInput (Game|GetPlayerController 0))
    (Variables|/Game/Characters/Player/BP_MyPlayer.BP_MyPlayer_C|SetGameMessage (Variables|Default|GetPlayerRef) "Press F To Interact")
    (else
      (Variables|/Game/Characters/Player/BP_MyPlayer.BP_MyPlayer_C|SetGameMessage (Variables|Default|GetPlayerRef) "Missing Keycard"))))

(event OnComponentEndOverlap(Box)
  (params (OverlappedComponent :type Primitive%20Component%20Object%20Reference) (OtherActor :type Actor%20Object%20Reference) (OtherComp :type Primitive%20Component%20Object%20Reference) (OtherBodyIndex :type Integer))
  ;[1 1 1] On end overlap stop displaying message and disable interact
  (bind _asbp_my_player (Utilities|Casting|CastToBP_MyPlayer OtherActor))
  (Variables|Default|SetPlayerRef _asbp_my_player)
  (Input|DisableInput (Game|GetPlayerController 0))
  (Variables|/Game/Characters/Player/BP_MyPlayer.BP_MyPlayer_C|SetGameMessage (Variables|Default|GetPlayerRef) "")
  (bind _doorslide (Timeline|DoorAnimation Reverse)
    (:Update
      (Transformation|SetRelativeLocation (Variables|Default|GetProxDoorMesh) _doorslide false false))))

(event Input|ActionEvents|InputActionInteract
  (params (Key :type Key%20Structure :default "None"))
  ;[1 1 1] On end overlap stop displaying message and disable interact
  (:Pressed
    (Audio|PlaySound2D "/Game/Assets/Audio/SFX/Door/creak3.creak3" 1.0 1.0 0.0 0 0)
    (bind _doorslide (Timeline|DoorAnimation Play)
      (:Update
        (Transformation|SetRelativeLocation (Variables|Default|GetProxDoorMesh) _doorslide false false)))))

(fn ConstructionScript)