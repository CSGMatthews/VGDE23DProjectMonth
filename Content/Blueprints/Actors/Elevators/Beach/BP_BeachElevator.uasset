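; BP_BeachElevator is an elevator actor that moves its lift when the player steps into a trigger box.
; Overlap with BP_MyPlayer plays the ElevatorLift timeline after a short delay, lerping LiftMesh's relative location from StartPoint to EndPoint.
; Leaving the box reverses the timeline after a longer delay, returning the lift toward its start.
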(event OnComponentBeginOverlap(Box)
  (params (OverlappedComponent :type Primitive%20Component%20Object%20Reference) (OtherActor :type Actor%20Object%20Reference) (OtherComp :type Primitive%20Component%20Object%20Reference) (OtherBodyIndex :type Integer) (bFromSweep :type Boolean) (SweepResult :type Hit%20Result%20Structure%20%28by%20ref%29))
  (Utilities|Casting|CastToBP_MyPlayer OtherActor)
  (Utilities|FlowControl|Delay 0.2)
  (bind _elevator_speed_ (Timeline|Elevator%20Lift Play)
    (:Update
      (Transformation|SetRelativeLocation (Variables|Default|GetLift_Mesh) (Math|Vector|Lerp(Vector) (Variables|Default|GetStart%20Point) (Variables|Default|GetEnd%20Point) _elevator_speed_) false false))))

(event OnComponentEndOverlap(Box)
  (params (OverlappedComponent :type Primitive%20Component%20Object%20Reference) (OtherActor :type Actor%20Object%20Reference) (OtherComp :type Primitive%20Component%20Object%20Reference) (OtherBodyIndex :type Integer))
  (Utilities|Casting|CastToBP_MyPlayer OtherActor)
  (Utilities|FlowControl|Delay 1.0)
  (bind _elevator_speed_ (Timeline|Elevator%20Lift Reverse)
    (:Update
      (Transformation|SetRelativeLocation (Variables|Default|GetLift_Mesh) (Math|Vector|Lerp(Vector) (Variables|Default|GetStart%20Point) (Variables|Default|GetEnd%20Point) _elevator_speed_) false false))))

(fn ConstructionScript)