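; Switch-operated elevator base actor that the player raises or lowers with the Interact input while inside its trigger box.
; Box overlap with BP_MyPlayer toggles actor input and sets or clears the player's interaction prompt.
; Pressing Interact plays a timeline that lerps LiftMesh between start and end points; releasing reverses it.
; A control flag gates both inputs until travel finishes, so a release mid-travel is ignored.
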(event OnComponentBeginOverlap(Box)
  (params (OverlappedComponent :type Primitive%20Component%20Object%20Reference) (OtherActor :type Actor%20Object%20Reference) (OtherComp :type Primitive%20Component%20Object%20Reference) (OtherBodyIndex :type Integer) (bFromSweep :type Boolean) (SweepResult :type Hit%20Result%20Structure%20%28by%20ref%29))
  ;[1 1 1] Overlaps
  (bind _asbp_my_player (Utilities|Casting|CastToBP_MyPlayer OtherActor))
  (Input|EnableInput (Game|GetPlayerController 0))
  (Variables|/Game/Blueprints/Characters/Player/BP_MyPlayer.BP_MyPlayer_C|SetGameMessage _asbp_my_player "Press F To Interact"))

(event OnComponentEndOverlap(Box)
  (params (OverlappedComponent :type Primitive%20Component%20Object%20Reference) (OtherActor :type Actor%20Object%20Reference) (OtherComp :type Primitive%20Component%20Object%20Reference) (OtherBodyIndex :type Integer))
  ;[1 1 1] Overlaps
  (bind _asbp_my_player (Utilities|Casting|CastToBP_MyPlayer OtherActor))
  (Input|DisableInput (Game|GetPlayerController 0))
  (Variables|/Game/Blueprints/Characters/Player/BP_MyPlayer.BP_MyPlayer_C|SetGameMessage _asbp_my_player " "))

(event Input|ActionEvents|InputActionInteract
  (params (Key :type Key%20Structure))
  (:Released
    (if (Variables|Default|Getb_CanControl)
      (Variables|Default|Setb_CanControl false)
      (bind _newtrack_0 (Timeline|Elevator%20Lift Reverse)
        (:Update
          (Transformation|SetRelativeLocation (Variables|Default|GetLift_Mesh) (Math|Vector|Lerp(Vector) (Variables|Default|Getv_Start%20Point) (Variables|Default|Getv_End%20Point) _newtrack_0) false false))
        (:Finished
          (Variables|Default|Setb_CanControl true))))))

(event Input|ActionEvents|InputActionInteract
  (params (Key :type Key%20Structure))
  (:Pressed
    (if (Variables|Default|Getb_CanControl)
      (Variables|Default|Setb_CanControl false)
      (bind _newtrack_0 (Timeline|Elevator%20Lift Play)
        (:Update
          (Transformation|SetRelativeLocation (Variables|Default|GetLift_Mesh) (Math|Vector|Lerp(Vector) (Variables|Default|Getv_Start%20Point) (Variables|Default|Getv_End%20Point) _newtrack_0) false false))
        (:Finished
          (Variables|Default|Setb_CanControl true))))))

(fn ConstructionScript)