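; Base chase enemy that pursues the player, deals contact damage and can drop a health pickup.
; BeginPlay sets a zero-interval looping timer intended for random navmesh wandering, while PawnSensing sends it after BP_MyPlayer via AIMoveTo.
; Sphere overlap damages the player through Ultimaki_GameInstance, gated by a DoOnce with delayed reset.
; Taking damage plays a flinch montage, or at zero health triggers effects, destruction and a random BP_Health_POW drop.
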(event OnSeePawn(PawnSensing)
  (params (Pawn :type Pawn%20Object%20Reference))
  ;[1 1 1] On Pawn Sence Chase the Player
  (bind _asbp_my_player (Utilities|Casting|CastToBP_MyPlayer Pawn))
  (bind _output_get (Variables|Character|SetPlayerReference _asbp_my_player))
  (AI|AIMoveTo self "0, 0, 0" _output_get 5.0 false))

(event OnComponentBeginOverlap(Sphere)
  (params (OverlappedComponent :type Primitive%20Component%20Object%20Reference) (OtherActor :type Actor%20Object%20Reference) (OtherComp :type Primitive%20Component%20Object%20Reference) (OtherBodyIndex :type Integer) (bFromSweep :type Boolean) (SweepResult :type Hit%20Result%20Structure%20%28by%20ref%29))
  ;[1 1 1] Attack Damage
  (Utilities|Casting|CastToBP_MyPlayer OtherActor)
  (Utilities|FlowControl|DoOnce false :!label _label
    (:Completed
      (bind _asultimaki_game_instance (Utilities|Casting|CastToUltimaki_GameInstance (Game|GetGameInstance)))
      (Default|TakeDamage _asultimaki_game_instance 1)
      (Utilities|FlowControl|Delay 3.0)
      (goto _label Reset))))

(event Custom|StartRandomLocation
  (Utilities|Time|SetTimerbyEvent (delegate Custom|FindRandomLocation) 0.0 true)
  (Development|PrintString "RandomLocation"))

(event Custom|FindRandomLocation
  (bind _self self)
  ;[1 1 1] On Begin play  Look for random location
  (AI|AIMoveTo _self (.RandomLocation (Class|NavigationSystemV1|GetRandomPointinNavigableRadius (Transformation|GetActorLocation) 1e+03 0 0)) _self 5.0 false
    (:then
      (Development|PrintString "Hello"))))

(event Custom|TakeDamage
  (params (Damage :type Integer))
  ;[1 1 1] On take any damage if they have health flinch if not kill them
  (bind _output_get (Variables|Default|SetI_EnemyHealth (- (Variables|Default|GetI_EnemyHealth) Damage)))
  (if (<= _output_get 0)
    (Audio|PlaySound2D 0 1.0 1.0 0.0 0 0)
    (Effects|SpawnEmitteratLocation 0 "0, 0, 0")
    (Utilities|FlowControl|Delay 0.2)
    (Actor|DestroyActor)
    (Game|SpawnActorfromClass (Utilities|Select :Index (Math|Random|RandomIntegerinRange 0 4) :Option%200 "/Game/Blueprints/Actors/PowerUps/BP_Health_POW.BP_Health_POW_C" :Option%201 0 :Option%202 0 :Option%203 0 :Option%204 0) (Math|Transform|MakeTransform (Transformation|GetActorLocation) "0, 0, 0" "1,1,1") "AlwaysSpawn" 0 0)
    (else
      (Audio|PlaySound2D 0 1.0 1.0 0.0 0 0)
      (Animation|Montage|PlayMontage (Variables|Character|GetMesh) 0))))

(event EventBeginPlay
  ;[1 1 1] On take any damage if they have health flinch if not kill them
  (CallFunction|StartRandomLocation))

(fn ConstructionScript)