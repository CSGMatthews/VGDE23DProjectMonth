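; Checkpoint actor that saves the player's position when BP_MyPlayer enters its box trigger.
; On overlap it loads the existing checkpoint save slot, or creates a new SGBP_CheckPointSave object if none exists.
; It stores the player's location as the last checkpoint location, writes the save back to the slot and prints the result.
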(event OnComponentBeginOverlap(Box)
  (params (OverlappedComponent :type Primitive%20Component%20Object%20Reference) (OtherActor :type Actor%20Object%20Reference) (OtherComp :type Primitive%20Component%20Object%20Reference) (OtherBodyIndex :type Integer) (bFromSweep :type Boolean) (SweepResult :type Hit%20Result%20Structure%20%28by%20ref%29))
  (bind _asbp_my_player (Utilities|Casting|CastToBP_MyPlayer OtherActor))
  (Variables|Default|Setv_Location (Transformation|GetActorLocation _asbp_my_player))
  (bind _returnvalue (SaveGame|DoesSaveGameExist "CheckpointSlot"))
  (if _returnvalue
    (bind _returnvalue_2 (SaveGame|LoadGamefromSlot "CheckpointSlot"))
    (bind _output_get (Variables|Default|SetSaverSubClass _returnvalue_2))
    (bind _assgbp_check_point_save (Utilities|Casting|CastToSGBP_CheckPointSave _output_get))
    (Variables|/Game/Blueprints/SavedGame/SGBP_CheckPointSave.SGBP_CheckPointSave_C|Setv_LastLocation _assgbp_check_point_save (Variables|Default|Getv_Location))
    (bind _returnvalue_3 (SaveGame|SaveGametoSlot (Variables|Default|GetSaverSubClass) "CheckpointSlot"))
    (Development|PrintString (Utilities|String|ToString(Boolean) _returnvalue_3))
    (else
      (bind _returnvalue_4 (SaveGame|CreateSaveGameObject "/Game/Blueprints/SavedGame/SGBP_CheckPointSave.SGBP_CheckPointSave_C"))
      (bind _output_get_2 (Variables|Default|SetSaverSubClass _returnvalue_4))
      (bind _assgbp_check_point_save_2 (Utilities|Casting|CastToSGBP_CheckPointSave _output_get_2))
      (Variables|/Game/Blueprints/SavedGame/SGBP_CheckPointSave.SGBP_CheckPointSave_C|Setv_LastLocation _assgbp_check_point_save_2 (Variables|Default|Getv_Location))
      (bind _returnvalue_5 (SaveGame|SaveGametoSlot (Variables|Default|GetSaverSubClass) "CheckpointSlot"))
      (Development|PrintString (Utilities|String|ToString(Boolean) _returnvalue_5)))))

(event EventBeginPlay)

(event Collision|EventActorBeginOverlap
  (params (OtherActor :type Actor%20Object%20Reference)))

(event EventTick
  (params (DeltaSeconds :type Float%20%28single-precision%29)))

(fn ConstructionScript)