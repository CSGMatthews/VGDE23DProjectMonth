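; Game Instance for Ultimaki that holds player lives, health, jump count and key cards, and handles damage, death and saving.
; TakeDamage plays hit feedback, updates the HUD and calls LifeLost at zero health.
; LifeLost either reloads the current level with refilled health or, on the last life, pauses into the game-over screen.
; Save, load, auto-save and clear functions persist stats and current level through a SGBP_MySavedGame slot.
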(event Custom|LifeLost
  (bind _returnvalue (Game|GetPlayerController 0))
  (bind _bp_playerref (Variables|Default|Getbp_PlayerRef))
  ;[1 1 1] LifeLost
  (bind _result (Math|Integer|DecrementInt (Variables|Default|Geti_PlayerLives))
    (:%20%20
      (if (== _result 0)
        (Input|DisableInput (Game|GetPlayerCharacter 0) (Game|GetPlayerController 0))
        (CameraFades|StartCameraFade (Game|GetPlayerCameraManager 0) 0.0 0.5 2.0 "(R=1.000000,G=0.000000,B=0.000000,A=1.000000)" false false)
        (Audio|PlaySound2D "/Game/Assets/Audio/Mario/29_Game_Over.29_Game_Over" 1.0 1.0 0.0 0 0)
        (Utilities|FlowControl|Delay 0.5)
        (bind _returnvalue_2 (UserInterface|CreateWidget "/Game/Blueprints/Widgets/GameOver/BP_GameOverScreen_w.BP_GameOverScreen_w_C"))
        (Widget|RemovefromParent (Variables|Default|Getbp_HUDReference))
        (UserInterface|Viewport|AddtoViewport _returnvalue_2 1)
        (Input|SetInputModeUIOnly _returnvalue _returnvalue_2 "DoNotLock")
        (Game|SetGamePaused true)
        (Variables|/Script/Engine.PlayerController|SetbShowMouseCursor _returnvalue true)
        (Actor|DestroyActor (Variables|Default|Getbp_PlayerRef))
        (else
          (Effects|SpawnEmitteratLocation "/Game/Assets/Particles/FX_Combat/WeaponCombo/P_ComboFinish_Tap_01.P_ComboFinish_Tap_01" (Transformation|GetWorldLocation (Variables|/Game/Characters/Player/BP_MyPlayer.BP_MyPlayer_C|GetBody (Variables|Default|Getbp_PlayerRef))))
          (Collision|SetActorEnableCollision _bp_playerref false)
          (Pawn|Components|CharacterMovement|DisableMovement (Variables|/Script/Engine.Character|GetCharacterMovement _bp_playerref))
          (Audio|SpawnSound2D "/Game/Assets/Audio/Mario/28_Player_Down.28_Player_Down" 1.0 1.0 0.0 0)
          (Utilities|FlowControl|Delay 3.0)
          (bind _returnvalue_3 (Game|GetCurrentLevelName true))
          (Game|OpenLevel(byName) (Utilities|String|StringToName _returnvalue_3))
          (Variables|Default|Seti_PlayerHealth 5)
          (Default|UpdateHealth (Variables|Default|Getbp_HUDReference)))))))

(event Custom|Reset
  ;[1 1 1] Reset the Game Stats back to default on called
  (Variables|Default|Seti_PlayerLives 3)
  (Variables|Default|Seti_PlayerHealth 5)
  (Variables|Default|Seti_JumpTimes 2)
  (Utilities|Array|Clear (Variables|Default|Getb_KeyCards?)))

(event Custom|TakeDamage
  (params (DamageTaken :type Integer))
  (bind _returnvalue (Math|Random|RandomFloatinRange 0.8 1.0))
  ;[1 1 1] Take Damage when called
  (Variables|Default|Seti_PlayerHealth (- (Variables|Default|Geti_PlayerHealth) DamageTaken))
  (Audio|PlaySound2D "/Game/Assets/Audio/SFX/Explosion1__004.Explosion1__004" _returnvalue _returnvalue 0.0 0 0)
  (Effects|SpawnEmitterAttached "/Game/Assets/Particles/FX_Ability/Stun/P_Stun_Stars_Base.P_Stun_Stars_Base" (Variables|/Game/Characters/Player/BP_MyPlayer.BP_MyPlayer_C|GetHurt (Variables|Default|Getbp_PlayerRef)) "None" "0, 0, 0" "0, 0, 0" "1.000000,1.000000,1.000000" "SnapToTargetIncludingScale")
  (bind _asultimaki_game_mode (Utilities|Casting|CastToUltimakiGameMode (Game|GetGameMode)))
  (Default|UpdateHealth (Variables|/Game/Blueprints/GameModes/UltimakiGameMode.UltimakiGameMode_C|GetHUD _asultimaki_game_mode))
  (if (<= (Variables|Default|Geti_PlayerHealth) 0)
    (bind _asultimaki_game_instance (Utilities|Casting|CastToUltimaki_GameInstance (Game|GetGameInstance)))
    (CallFunction|LifeLost _asultimaki_game_instance)))

(event EventInit
  (bind _returnvalue (SaveGame|CreateSaveGameObject "/Game/Blueprints/GameModes/SGBP_MySavedGame.SGBP_MySavedGame_C"))
  (Variables|Default|SetSaveGameData _returnvalue))

(fn SetPlayerRef
  (params (PlayerRef :type BP%20My%20Player%20Object%20Reference))
  (Variables|Default|Setbp_PlayerRef PlayerRef))

(fn SavePlayerData
  (bind _returnvalue (Game|GetCurrentLevelName true))
  (Variables|/Game/Blueprints/GameModes/SGBP_MySavedGame.SGBP_MySavedGame_C|SetBP_PlayerData (Variables|Default|GetSaveGameData) (Utilities|Struct|MakeBPS_PlayerSaveData (Variables|Default|Geti_JumpTimes) (Variables|Default|Geti_PlayerHealth) (Variables|Default|Geti_PlayerLives) (Variables|Default|Getb_KeyCards?) (Utilities|String|StringToName _returnvalue)))
  (SaveGame|SaveGametoSlot (Variables|Default|GetSaveGameData) (Variables|Default|Gets_SaveSlotName)))

(fn LoadPlayerData
  (bind _returnvalue (SaveGame|LoadGamefromSlot (Variables|Default|Gets_SaveSlotName)))
  (bind _assgbp_my_saved_game (Utilities|Casting|CastToSGBP_MySavedGame _returnvalue))
  (bind _output_get (Variables|Default|SetSaveGameData _assgbp_my_saved_game))
  (Game|OpenLevel(byName) (.currentlevel (Variables|/Game/Blueprints/GameModes/SGBP_MySavedGame.SGBP_MySavedGame_C|GetBP_PlayerData _output_get)))
  (Variables|Default|Seti_JumpTimes (.jumptimes (Variables|/Game/Blueprints/GameModes/SGBP_MySavedGame.SGBP_MySavedGame_C|GetBP_PlayerData _output_get)))
  (Variables|Default|Seti_PlayerHealth (.playerhealth (Variables|/Game/Blueprints/GameModes/SGBP_MySavedGame.SGBP_MySavedGame_C|GetBP_PlayerData _output_get)))
  (Variables|Default|Seti_PlayerLives (.playerlifes (Variables|/Game/Blueprints/GameModes/SGBP_MySavedGame.SGBP_MySavedGame_C|GetBP_PlayerData _output_get)))
  (Variables|Default|Setb_KeyCards? (.keycards (Variables|/Game/Blueprints/GameModes/SGBP_MySavedGame.SGBP_MySavedGame_C|GetBP_PlayerData _output_get))))

(fn ClearSaveData
  (SaveGame|DeleteGameinSlot (Variables|Default|Gets_SaveSlotName)))

(fn AutoSave
  (CallFunction|SavePlayerData))