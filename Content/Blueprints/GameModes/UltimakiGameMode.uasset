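; UltimakiGameMode is a game mode that sets up the HUD and runs a countdown timer for play.
; On BeginPlay it creates the HUD widget, updates its health display, stores its reference in the game instance and resets the timer to base values.
; A looping one-second timer decrements seconds and rolls over minutes; when time runs out, it calls LifeLost on the game instance and clears itself.
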(event Custom|TimerTick
  ;[1 1 1] Timer for game
  (bind _result (Math|Float|DecrementFloat (Variables|Default|Getf_Seconds))
    (:%20%20
      (if (< _result 0.0)
        (bind _result_2 (Math|Float|DecrementFloat (Variables|Default|Getf_Minutes))
          (:%20%20
            (if (< _result_2 0.0)
              (Variables|Default|Setf_Minutes 0.0)
              (Variables|Default|Setf_Seconds 0.0)
              (bind _asultimaki_game_instance (Utilities|Casting|CastToUltimaki_GameInstance (Game|GetGameInstance)))
              (Default|LifeLost _asultimaki_game_instance)
              (Utilities|Time|ClearandInvalidateTimerbyHandle (Variables|Default|GetTimerHandle))
              (else
                (Variables|Default|Setf_Seconds 59.0)))))))))

(event EventBeginPlay
  (Utilities|FlowControl|Sequence
    (:then_0
      ;[1 1 1] Create Heads Up Display
      (bind _returnvalue (UserInterface|CreateWidget "/Game/Blueprints/Widgets/HUD/BP_HeadsUpDisplay_w.BP_HeadsUpDisplay_w_C"))
      (bind _output_get (Variables|Default|SetHUD _returnvalue))
      (UserInterface|Viewport|AddtoViewport _output_get 0)
      (Default|UpdateHealth _returnvalue)
      (bind _asultimaki_game_instance (Utilities|Casting|CastToUltimaki_GameInstance (Game|GetGameInstance)))
      (Variables|/Game/Blueprints/GameModes/Ultimaki_GameInstance.Ultimaki_GameInstance_C|Setbp_HUDReference _asultimaki_game_instance (Variables|Default|GetHUD))
      (Variables|/Game/Blueprints/GameModes/Ultimaki_GameInstance.Ultimaki_GameInstance_C|Seti_PlayerLives _asultimaki_game_instance (Variables|/Game/Blueprints/GameModes/Ultimaki_GameInstance.Ultimaki_GameInstance_C|Geti_PlayerLives _asultimaki_game_instance))
      (Development|PrintString "GameMode"))
    (:then_1
      ;[1 1 1] Reset timer to default
      (Variables|Default|Setf_Minutes (Variables|Default|Getf_BaseMinutes))
      (Variables|Default|Setf_Seconds (Variables|Default|Getf_BaseSeconds)))
    (:then_2
      (bind _returnvalue_2 (Utilities|Time|SetTimerbyEvent (delegate Custom|TimerTick) 1.0 true))
      (Variables|Default|SetTimerHandle _returnvalue_2))))

(fn ConstructionScript)